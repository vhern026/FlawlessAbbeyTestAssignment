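; GM_TestDemo is the game mode for a test demo, setting up the HUD and bridging inventory data between the game instance and the UI.
; On BeginPlay it copies Items from GI_TestDemo, creates WBP_HUD, caches the BP_Player character, then loads the items into the HUD's inventory widget.
; LoadInventory pushes the current Items to that widget again, while UpdateInventoryData writes them back to the game instance.
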(event EventBeginPlay
  (bind _asgi_test_demo (Utilities|Casting|CastToGI_TestDemo (Game|GetGameInstance)))
  (Variables|Default|SetGameInstance _asgi_test_demo)
  (Variables|Default|SetItems (Variables|/Game/Blueprints/GI_TestDemo.GI_TestDemo_C|GetItems (Variables|Default|GetGameInstance)))
  (bind _returnvalue (UserInterface|CreateWidget "/Game/UI/Widgets/WBP_HUD.WBP_HUD_C" (Game|GetPlayerController 0)))
  (bind _output_get (Variables|Default|SetHUDWidget _returnvalue))
  (UserInterface|Viewport|AddtoViewport _output_get 1)
  (bind _asbp_player (Utilities|Casting|CastToBP_Player (Game|GetPlayerCharacter 0)))
  (Variables|Default|SetPlayer _asbp_player)
  (Default|LoadInventory (Variables|/Game/UI/Widgets/WBP_HUD.WBP_HUD_C|GetWBP_Inventory (Variables|Default|GetHUDWidget)) (Variables|Default|GetItems))
  (Default|LoadViewport (Variables|/Game/UI/Widgets/WBP_HUD.WBP_HUD_C|GetWBP_Inventory (Variables|Default|GetHUDWidget))))

(event EventTick
  (params (DeltaSeconds :type Float%20%28single-precision%29)))

(fn ConstructionScript)

(fn LoadInventory
  (Default|LoadInventory (Variables|/Game/UI/Widgets/WBP_HUD.WBP_HUD_C|GetWBP_Inventory (Variables|Default|GetHUDWidget)) (Variables|Default|GetItems)))

(fn UpdateInventoryData
  (Variables|/Game/Blueprints/GI_TestDemo.GI_TestDemo_C|SetItems (Variables|Default|GetGameInstance) (Variables|Default|GetItems)))