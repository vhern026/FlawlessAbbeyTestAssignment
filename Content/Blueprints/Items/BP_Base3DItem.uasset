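; Base pickup item that loads its properties from a data table and joins the player's inventory on interaction.
; Interacting switches to a dialogue camera, locks interaction and writes the item into the first GameMode slot that can stack it (64 cap) or is empty.
; DT_Dialogue rows chain through NextRow to feed HUD dialogue.
; Finishing restores the player and destroys the item unless cutscene-locked, then updates persistent inventory.
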(event EventInteract
  (params (Instigator :type BP%20Character%20Base%20Object%20Reference))
  (if (!= (Variables|Properties|GetCurrentRowName) "")
    (Interaction|StartCharacterInteraction Instigator)
    (Interaction|StartInteraction Instigator)
    (Utilities|FlowControl|Delay 0.2)
    (Interaction|ShowDialogueLine)
    (else
      (Audio|PlaySound2D "/Engine/VREditor/Sounds/UI/Click_on_Button.Click_on_Button" 1.0 1.0 0.0 0 0))))

(event EventFinishInteraction
  (Interaction|EndInteraction)
  (Default|UpdatePersistentInventory (Variables|Properties|GetGameMode)))

(event EventBeginPlay
  (Rendering|SetCastShadow (Variables|Default|GetInteractionIndicator) false)
  (Variables|Properties|SetResetRowName (Variables|Properties|GetCurrentRowName))
  (bind _asgm_test_demo (Utilities|Casting|CastToGM_TestDemo (Game|GetGameMode)))
  (Variables|Properties|SetGameMode _asgm_test_demo)
  (bind _asgi_test_demo (Utilities|Casting|CastToGI_TestDemo (Game|GetGameInstance)))
  (Variables|Properties|SetGameInstance _asgi_test_demo)
  (Setter|SetItem (Variables|Inventory|GetTableRowName)))

(fn ConstructionScript)

(fn StartInteraction
  (params (InteractInstigator :type Actor%20Object%20Reference))
  (bind _gamemode (Variables|Properties|GetGameMode))
  (Rendering|SetVisibility (Variables|Default|GetInteractionIndicator) false false)
  (Audio|PlaySound2D "/Engine/VREditor/Sounds/UI/Click_on_Button.Click_on_Button" 0.1 1.0 0.0 0 0)
  (bind _asbp_player (Utilities|Casting|CastToBP_Player InteractInstigator))
  (Default|ChangeCameraDialogue _asbp_player self)
  (Variables|/Game/Blueprints/Character/BP_CharacterBase.BP_CharacterBase_C|SetIsInteractionLocked _asbp_player true)
  (Setter|SetItemtoInventory)
  (Default|LoadInventory _gamemode)
  (Default|LoadViewport (Variables|/Game/UI/Widgets/WBP_HUD.WBP_HUD_C|GetWBP_Inventory (Variables|/Game/Blueprints/GM_TestDemo.GM_TestDemo_C|GetHUDWidget _gamemode))))

(fn HideDialogue
  (Variables|Properties|SetIsInteractionLocked true)
  (Audio|PlaySound2D "/Engine/VREditor/Sounds/UI/Click_on_Button.Click_on_Button" 0.1 1.0 0.0 0 0))

(fn EndInteraction
  (Rendering|SetVisibility (Variables|Default|GetInteractionIndicator) true false)
  (bind _asbp_player (Utilities|Casting|CastToBP_Player (Game|GetPlayerCharacter 0)))
  (if (not (Variables|/Game/Blueprints/Character/BP_Player.BP_Player_C|GetIsCutsceneLocked _asbp_player))
    (bind _asbp_player_2 (Utilities|Casting|CastToBP_Player (Game|GetPlayerCharacter 0)))
    (Default|ChangeCameraDialogue _asbp_player_2 _asbp_player_2)
    (Variables|/Game/Blueprints/Character/BP_CharacterBase.BP_CharacterBase_C|SetIsInteractionLocked _asbp_player_2 false)
    (Actor|DestroyActor)))

(fn ShowDialogueLine
  (bind _gamemode (Variables|Properties|GetGameMode))
  (bind _returnvalue (Utilities|GetDataTableRow "/Game/DataTable/Dialogue/DT_Dialogue.DT_Dialogue" (Variables|Properties|GetCurrentRowName))
    (:then
      (Default|ShowDialogue (Variables|/Game/Blueprints/GM_TestDemo.GM_TestDemo_C|GetHUDWidget _gamemode) (Variables|/Game/Blueprints/GM_TestDemo.GM_TestDemo_C|GetPlayer _gamemode) (Variables|Properties|GetName) (.DialogueText (Utilities|Struct|BreakS_Dialogue _returnvalue)))
      (Variables|Properties|SetNextRow (.NextRow (Utilities|Struct|BreakS_Dialogue _returnvalue)))
      (return))))

(fn StartCharacterInteraction
  (params (Player :type Actor%20Object%20Reference))
  (if (Variables|Properties|GetIsInteractable)
    (bind _asbp_player (Utilities|Casting|CastToBP_Player Player))
    (Default|StartInteraction _asbp_player (Actor|GetParentActor _asbp_player))))

(fn SetItemtoInventory
  (bind (_array_element _array_index) (Utilities|Array|ForEachLoopwithBreak (Variables|/Game/Blueprints/GM_TestDemo.GM_TestDemo_C|GetItems (Variables|Properties|GetGameMode)) :!label _label)
    (:LoopBody
      (bind (_item_name _amount) (Getter|GetItemProperties))
      (Variables|Inventory|SetInventoryArrayIndex _array_index)
      (if (and (Utilities|Enum|Equal(Enum) _item_name (.ItemName (Utilities|Struct|BreakS_ItemProperties _array_element))) (<= (+ _amount (.Amount (Utilities|Struct|BreakS_ItemProperties _array_element))) 64))
        (bind (_item_name_2 _amount_2 _item _itemimage) (Getter|GetItemProperties))
        (Utilities|Array|SetArrayElem (Variables|/Game/Blueprints/GM_TestDemo.GM_TestDemo_C|GetItems (Variables|Properties|GetGameMode)) (Variables|Inventory|GetInventoryArrayIndex) (Utilities|Struct|MakeS_ItemProperties _item_name_2 (+ _amount (.Amount (Utilities|Struct|BreakS_ItemProperties _array_element))) _itemimage))
        (Variables|Inventory|SetInventoryArrayIndex 0)
        (goto _label Break)
        (elif (<= (.Amount (Utilities|Struct|BreakS_ItemProperties _array_element)) 0)
          (bind _item_2 (Getter|GetItemProperties))
          (Utilities|Array|SetArrayElem (Variables|/Game/Blueprints/GM_TestDemo.GM_TestDemo_C|GetItems (Variables|Properties|GetGameMode)) (Variables|Inventory|GetInventoryArrayIndex) _item_2)
          (Variables|Inventory|SetInventoryArrayIndex 0)
          (goto _label Break))))))

(fn SetItem
  (params (RowName :type Name))
  (bind _returnvalue (Utilities|GetDataTableRow (Variables|Inventory|GetDT_Item) RowName)
    (:then
      (Variables|Inventory|SetItem _returnvalue))))

(fn GetItemProperties
  (bind _item (Variables|Inventory|GetItem))
  (bind (_itemname _amount _itemimage) (Utilities|Struct|BreakS_ItemProperties _item))
  (return _itemname _amount (Variables|Inventory|GetItem) _itemimage))

(fn GetInventory
  (return (Variables|/Game/Blueprints/GM_TestDemo.GM_TestDemo_C|GetItems (Variables|Properties|GetGameMode))))

(fn ShowNextLine
  (if (Utilities|Array|IsEmpty (Variables|Properties|GetNextRow))
    (Variables|Properties|SetCurrentRowName (Variables|Properties|GetResetRowName))
    (return false)
    (else
      (Variables|Properties|SetCurrentRowName (Utilities|String|StringToName (Variables|Properties|GetNextRow)))
      (Interaction|ShowDialogueLine)
      (Audio|PlaySound2D "/Engine/VREditor/Sounds/UI/Click_on_Button.Click_on_Button" 1.0 1.0 0.0 0 0)
      (return true))))