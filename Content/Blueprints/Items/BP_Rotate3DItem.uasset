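; Item actor that renders a rotatable, zoomable 3D preview of an item mesh via a scene capture limited to its own components.
; UpdateStaticMesh applies the mesh and camera setup from recording settings.
; Each Tick, game mode X, Y and zoom values rotate and move the SceneCaptureComponentCube.
; It also loads item data from a data table and adds it to the game mode's inventory, stacking up to 64 or filling an empty slot.
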(event EventTick
  (params (DeltaSeconds :type Float%20%28single-precision%29))
  (bind _gamemode (Variables|Properties|GetGameMode))
  (CallFunction|UpdateCameraRotation (Variables|/Game/Blueprints/GM_TestDemo.GM_TestDemo_C|GetItem3DX _gamemode) (Variables|/Game/Blueprints/GM_TestDemo.GM_TestDemo_C|GetItem3DY _gamemode))
  (CallFunction|UpdateCameraPosition (Variables|/Game/Blueprints/GM_TestDemo.GM_TestDemo_C|GetItem3DZoomZ _gamemode)))

(event EventBeginPlay
  (Rendering|SceneCapture|ShowOnlyActorComponents (Variables|Default|GetSceneCaptureComponent2D) self false)
  (bind _asgm_test_demo (Utilities|Casting|CastToGM_TestDemo (Game|GetGameMode)))
  (Variables|Properties|SetGameMode _asgm_test_demo)
  (bind _asgi_test_demo (Utilities|Casting|CastToGI_TestDemo (Game|GetGameInstance)))
  (Variables|Properties|SetGameInstance _asgi_test_demo))

(fn ConstructionScript)

(fn SetItemtoInventory
  (bind (_array_element _array_index) (Utilities|Array|ForEachLoopwithBreak (Variables|/Game/Blueprints/GM_TestDemo.GM_TestDemo_C|GetItems (Variables|Properties|GetGameMode)) :!label _label)
    (:LoopBody
      (bind (_item_name _amount) (Getter|GetItemProperties))
      (Variables|Inventory|SetInventoryArrayIndex _array_index)
      (if (and (Utilities|Enum|Equal(Enum) _item_name (.ItemName (Utilities|Struct|BreakS_ItemProperties _array_element))) (<= (+ _amount (.Amount (Utilities|Struct|BreakS_ItemProperties _array_element))) 64))
        (bind (_item_name_2 _amount_2 _item _itemimage) (Getter|GetItemProperties))
        (Utilities|Array|SetArrayElem (Variables|/Game/Blueprints/GM_TestDemo.GM_TestDemo_C|GetItems (Variables|Properties|GetGameMode)) (Variables|Inventory|GetInventoryArrayIndex) (Utilities|Struct|MakeS_ItemProperties _item_name_2 (+ _amount (.Amount (Utilities|Struct|BreakS_ItemProperties _array_element))) _itemimage))
        (Variables|Inventory|SetInventoryArrayIndex 0)
        (goto _label Break)
        (elif (<= (.Amount (Utilities|Struct|BreakS_ItemProperties _array_element)) 0)
          (bind _item_2 (Getter|GetItemProperties))
          (Utilities|Array|SetArrayElem (Variables|/Game/Blueprints/GM_TestDemo.GM_TestDemo_C|GetItems (Variables|Properties|GetGameMode)) (Variables|Inventory|GetInventoryArrayIndex) _item_2)
          (Variables|Inventory|SetInventoryArrayIndex 0)
          (goto _label Break))))))

(fn SetItem
  (params (RowName :type Name))
  (bind _returnvalue (Utilities|GetDataTableRow (Variables|Inventory|GetDT_Item) RowName)
    (:then
      (Variables|Inventory|SetItem _returnvalue))))

(fn GetItemProperties
  (bind _item (Variables|Inventory|GetItem))
  (bind (_itemname _amount _itemimage) (Utilities|Struct|BreakS_ItemProperties _item))
  (return _itemname _amount (Variables|Inventory|GetItem) _itemimage))

(fn GetInventory
  (return (Variables|/Game/Blueprints/GM_TestDemo.GM_TestDemo_C|GetItems (Variables|Properties|GetGameMode))))

(fn UpdateStaticMesh
  (params (Recording3dSettings :type S%20Item%203D%20Settings%20Structure))
  (bind (_mesh _cameraposition _maxposition _minposition) (Utilities|Struct|BreakS_Item3DSettings Recording3dSettings))
  (if (!= _mesh 0)
    (Components|StaticMesh|SetStaticMesh (Variables|Default|GetItem3DViewMesh) _mesh)
    (Transformation|SetRelativeLocation (Variables|Default|GetSceneCaptureComponent2D) _cameraposition false false)
    (CallFunction|UpdateCameraRotation _maxposition _minposition)))

(fn UpdateCameraRotation
  (params (X :type Float%20%28double-precision%29) (Y :type Float%20%28double-precision%29))
  (Transformation|SetRelativeRotation (Variables|Default|GetSceneCaptureComponentCube) (Math|Rotator|MakeRotator X Y 0.0) false false)
  (return))

(fn ResetMesh
  (Components|StaticMesh|SetStaticMesh (Variables|Default|GetItem3DViewMesh) 0))

(fn UpdateCameraPosition
  (params (Z :type Float%20%28double-precision%29))
  (Transformation|SetRelativeLocation (Variables|Default|GetSceneCaptureComponentCube) (Math|Vector|MakeVector 0.0 0.0 Z) false false)
  (return))