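; NPC character Blueprint that adds camera, facing and indicator behavior to the dialogue interaction logic inherited from its parent.
; On BeginPlay it hides the interaction indicator if no dialogue row name is set.
; Starting an interaction switches the player's dialogue camera to the NPC, hides the indicator and yaws the NPC toward the instigator.
; Ending it shows the indicator again and returns the camera to the player.
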(event EventBeginPlay
  (|CallParentFunction)
  (if (== (Variables|Default|GetCurrentRowName) "")
    (Rendering|SetVisibility (Variables|Default|GetInteractionIndicator) false false)))

(event Collision|EventActorBeginOverlap
  (params (OtherActor :type Actor%20Object%20Reference)))

(event EventTick
  (params (DeltaSeconds :type Float%20%28single-precision%29)))

(fn ConstructionScript
  (|CallParentFunction))

(fn StartInteraction
  (params (InteractInstigator :type Actor%20Object%20Reference))
  (bind _returnvalue (Transformation|GetActorRotation))
  (bind _asbp_player (Utilities|Casting|CastToBP_Player InteractInstigator))
  (Default|ChangeCameraDialogue _asbp_player self)
  (|CallParentFunction InteractInstigator)
  (Rendering|SetVisibility (Variables|Default|GetInteractionIndicator) false false)
  (bind _interactinstigator (LocalVariables|GetInteractInstigator)
    (:then
      (Transformation|SetActorRotation (Math|Rotator|MakeRotator (.roll _returnvalue) (.pitch _returnvalue) (.yaw (Math|Rotator|FindLookatRotation (Transformation|GetActorLocation) (Transformation|GetActorLocation _interactinstigator))))))
    (:else)))

(fn EndInteraction
  (|CallParentFunction)
  (Rendering|SetVisibility (Variables|Default|GetInteractionIndicator) true false)
  (bind _asbp_player (Utilities|Casting|CastToBP_Player (Game|GetPlayerCharacter 0)))
  (Default|ChangeCameraDialogue _asbp_player _asbp_player))

(fn ShowDialogueLine
  (|CallParentFunction))