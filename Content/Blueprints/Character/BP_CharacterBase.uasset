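; Base character Blueprint that provides interaction and data-table-driven dialogue.
; Interact locks the character, stops its movement and, after a short delay, sends the current DT_Dialogue row to the GameMode's HUD widget.
; ShowNextLine follows each row's NextRow link, returning false and resetting to the starting row when the chain ends.
; FinishInteraction releases the lock unless BP_Player is cutscene-locked.
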(event EventInteract
  (params (Instigator :type BP%20Character%20Base%20Object%20Reference))
  ;[1 1 1] Display Dialogue through Interface
  (if (!= (Variables|Interaction|GetCurrentRowName) "")
    (CallFunction|StartInteraction Instigator)
    (CallFunction|StartInteraction Instigator)
    (Utilities|FlowControl|Delay 0.2)
    (CallFunction|ShowDialogueLine)
    (else
      (Audio|PlaySound2D "/Engine/VREditor/Sounds/UI/Click_on_Button.Click_on_Button" 1.0 1.0 0.0 0 0))))

(event EventBeginPlay
  (Rendering|SetCastShadow (Variables|Default|GetInteractionIndicator) false)
  (Variables|Interaction|SetResetRowName (Variables|Interaction|GetCurrentRowName))
  (bind _asgm_test_demo (Utilities|Casting|CastToGM_TestDemo (Game|GetGameMode)))
  (Variables|Default|SetGameMode _asgm_test_demo))

(event EventFinishInteraction
  ;[1 1 1] Ends the interaction, the rest is handled on BP Player
  (CallFunction|EndInteraction))

(fn ConstructionScript)

(fn ShowDialogueLine
  (bind _returnvalue (Utilities|GetDataTableRow "/Game/DataTable/Dialogue/DT_Dialogue.DT_Dialogue" (Variables|Interaction|GetCurrentRowName))
    (:then
      (Default|ShowDialogue (Variables|/Game/Blueprints/GM_TestDemo.GM_TestDemo_C|GetHUDWidget (Variables|Default|GetGameMode)) self (Variables|Interaction|GetName) (.DialogueText (Utilities|Struct|BreakS_Dialogue _returnvalue)))
      (Variables|Interaction|SetNextRow (.NextRow (Utilities|Struct|BreakS_Dialogue _returnvalue)))
      (return))))

(fn StartInteraction
  (params (InteractInstigator :type Actor%20Object%20Reference))
  (Variables|Interaction|SetIsInteractionLocked true)
  (Components|Movement|StopMovementImmediately (Variables|Character|GetCharacterMovement))
  (Audio|PlaySound2D "/Engine/VREditor/Sounds/UI/Click_on_Button.Click_on_Button" 0.1 1.0 0.0 0 0))

(fn EndInteraction
  (bind _asbp_player (Utilities|Casting|CastToBP_Player (Game|GetPlayerCharacter 0)))
  (if (not (Variables|/Game/Blueprints/Character/BP_Player.BP_Player_C|GetIsCutsceneLocked _asbp_player))
    (Variables|Interaction|SetIsInteractionLocked false)))

(fn HideDialogue
  (Variables|Interaction|SetIsInteractionLocked true)
  (Components|Movement|StopMovementImmediately (Variables|Character|GetCharacterMovement))
  (Audio|PlaySound2D "/Engine/VREditor/Sounds/UI/Click_on_Button.Click_on_Button" 0.1 1.0 0.0 0 0))

(fn ShowNextLine
  (if (Utilities|Array|IsEmpty (Variables|Interaction|GetNextRow))
    (Variables|Interaction|SetCurrentRowName (Variables|Interaction|GetResetRowName))
    (return false)
    (else
      (Variables|Interaction|SetCurrentRowName (Utilities|String|StringToName (Variables|Interaction|GetNextRow)))
      (CallFunction|ShowDialogueLine)
      (Audio|PlaySound2D "/Engine/VREditor/Sounds/UI/Click_on_Button.Click_on_Button" 1.0 1.0 0.0 0 0)
      (return true))))